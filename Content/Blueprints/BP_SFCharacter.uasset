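; BP_SFCharacter is a character Blueprint that tests attack animation montages with root motion.
; The Attack input alternates left and right slash montages through a FlipFlop, and the Kick input plays a kick montage.
; Both use the PlayMontageDelayed macro, which plays immediately, then closes a gate for the delay, so each call site ignores repeat presses during its own cooldown.
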(event EventBeginPlay)

(event Input|ActionEvents|InputActionAttack
  (params (Key :type Key%20Structure :default "None"))
  ;[1 1 1] Test Animation montages with root
  (:Pressed
    (Utilities|FlowControl|FlipFlop
      (:A
        (Utilities|PlayMontageDelayed 1.0 "/Game/Mixamo/RetargetRootAnim/fight/sf_attack_slash_L_Montage.sf_attack_slash_L_Montage"))
      (:B
        (Utilities|PlayMontageDelayed 1.0 "/Game/Mixamo/RetargetRootAnim/fight/sf_attack_slash_R_Montage.sf_attack_slash_R_Montage")))))

(event Input|ActionEvents|InputActionKick
  (params (Key :type Key%20Structure :default "None"))
  ;[1 1 1] Test Animation montages with root
  (:Pressed
    (Utilities|PlayMontageDelayed 1.0 "/Game/Mixamo/RetargetRootAnim/fight/sf_attack_kick_Montage.sf_attack_kick_Montage")))

(fn ConstructionScript)