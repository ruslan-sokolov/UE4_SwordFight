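; One-handed weapon Blueprint with a test attack that plays a right slash montage on its owning character.
; Attack_Test fires only when no montage is playing, simulates physics on all MeshComp bodies during the swing, and turns it off on completion or interruption, printing debug messages.
; A separate PlayCharacterMontageDelayed macro uses a gate and delay to rate-limit montage playback, though Attack_Test does not use it.
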(event Custom|Attack_Test
  (bind _ownedcharacter (Variables|Default|GetOwnedCharacter))
  (bind _meshcomp (Variables|Default|GetMeshComp))
  (Utilities|IsValid (Animation|GetCurrentMontage _ownedcharacter :!class /Script/Engine.Character)
    (:Is%20Not%20Valid
      (Animation|Montage|PlayMontage (Variables|/Script/Engine.Character|GetMesh _ownedcharacter) "/Game/Anims/RetargetRootAnim/fight/sf_attack_slash_R_Montage.sf_attack_slash_R_Montage"
        (:then
          (Class|SkeletalMeshComponent|SetAllBodiesSimulatePhysics _meshcomp true)
          (Development|PrintString "Axe Physic on" true true "(R=1.000000,G=0.402783,B=0.201510,A=1.000000)"))
        (:OnCompleted
          (Class|SkeletalMeshComponent|SetAllBodiesSimulatePhysics _meshcomp false :!label _label)
          (Development|PrintString "Axe Physic off" true true "(R=1.000000,G=0.092666,B=0.000000,A=1.000000)"))
        (:OnInterrupted
          (goto _label))))))

(fn ConstructionScript)